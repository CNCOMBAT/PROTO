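; Game instance for the multiplayer game that handles session hosting, quick play and main menu navigation.
; Hosting creates a LAN or online session and opens the Lobby level as a listen server.
; Quick Play searches LAN first, falls back to online if none is found, joins the first result and shows status on a loading-screen switcher.
; Menu events clear all widgets, then lazily create, cache and display the requested screen.
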(event `HostGame`
  (params (MaxPlayers :type Integer) (`Is Lan?` :type Boolean))
  ;[1 0 0.04893] Host Game
  (set `self.Hoster` true)
  (`CreateSessionCallbackProxy.CreateSession` (`GameplayStatics.GetPlayerController` 0) MaxPlayers `Is Lan?`
    (:`OnSuccess`
      (`GameplayStatics.OpenLevel` "Lobby" true "listen"))
    (:`OnFailure`
      (`KismetSystemLibrary.PrintString` "CREATE SESSION FAILED in MainGI" true true (struct :`R` 1.0 :`B` 0.084287 :`A` 1.0) 33.0))))

(event `ShowHomeMenu`
  ;[0 0.5871 1] MENU
  ;;[1 1 1] Display Home Menu Widget
  (`WidgetLayoutLibrary.RemoveAllWidgets`)
  (`/Engine/EditorBlueprintResources/StandardMacros.IsValid` (`self.HomeMenuWB`)
    (:`Is Valid`
      _)
    (:`Is Not Valid`
      (bind _returnvalue (`|CreateWidget` "/Game/MP_SK/UI/MainMenu/HomeMenu.HomeMenu_C" (`GameplayStatics.GetPlayerController` 0)))
      (bind _output_get (set `self.HomeMenuWB` _returnvalue))))
  (`UserWidget.AddToViewport` _output_get 0) ; And add the MainMenu to the Viewport
  (set `PlayerController.bShowMouseCursor` true (`GameplayStatics.GetPlayerController` 0)))

(event `QuickPlay`
  ;[0 1 0.0928] Quick Play. Connect to first found game
  (bind _returnvalue (`|CreateWidget` "/Game/MP_SK/UI/Lobby/AdditionalLobbyWidgets/QuickPlayLoadingScreen.QuickPlayLoadingScreen_C" (`GameplayStatics.GetPlayerController` 0)))
  ;;[1 1 1] First trying to find session in lan network
  (`UserWidget.AddToViewport` _returnvalue 0)
  (bind _results (`FindSessionsCallbackProxy.FindSessions` (`GameplayStatics.GetPlayerController` 0) 1 true)
    (:`OnSuccess`
      (if (!= (`KismetArrayLibrary.Array_Length` _results) 0)
        (set `self.FirstFoundSession` (`|GetArrayItem` _results))
        (bind _widgetswitcher_0 (`/Game/MP_SK/UI/Lobby/AdditionalLobbyWidgets/QuickPlayLoadingScreen.WidgetSwitcher_0` _returnvalue))
        (`WidgetSwitcher.SetActiveWidgetIndex` _widgetswitcher_0 2 :!label _label)
        (`KismetSystemLibrary.Delay` 1.0)
        (`JoinSessionCallbackProxy.JoinSession` (`GameplayStatics.GetPlayerController` 0) (`self.FirstFoundSession`))
        (else
          ;;[1 1 1] Second. Trying to find session in global network
          (bind _results_2 (`FindSessionsCallbackProxy.FindSessions` (`GameplayStatics.GetPlayerController` 0) 1)
            (:`OnSuccess`
              (if (!= (`KismetArrayLibrary.Array_Length` _results_2) 0)
                (set `self.FirstFoundSession` (`|GetArrayItem` _results_2))
                (goto _label)
                (else
                  (`WidgetSwitcher.SetActiveWidgetIndex` _widgetswitcher_0 1))))
            (:`OnFailure`
              (`WidgetSwitcher.SetActiveWidgetIndex` _widgetswitcher_0 3 :!label _label_2))))))
    (:`OnFailure`
      (goto _label_2))))

(event `ShowMultiplayerMenu`
  ;[0 0.5871 1] MENU
  ;;[1 1 1] Display Multiplayer Menu Widget
  (`WidgetLayoutLibrary.RemoveAllWidgets`)
  (`/Engine/EditorBlueprintResources/StandardMacros.IsValid` (`self.MultiplayerMenuWB`)
    (:`Is Valid`
      _)
    (:`Is Not Valid`
      (bind _returnvalue (`|CreateWidget` "/Game/MP_SK/UI/MainMenu/MultiplayerMenu.MultiplayerMenu_C" (`GameplayStatics.GetPlayerController` 0)))
      (bind _output_get (set `self.MultiplayerMenuWB` _returnvalue))))
  (`UserWidget.AddToViewport` _output_get 0) ; And add the MainMenu to the Viewport
)

(event `ShowHostGameMenu`
  ;[0 0.5871 1] MENU
  ;;[1 1 1] Display HostGame Menu Widget
  (`WidgetLayoutLibrary.RemoveAllWidgets`)
  (`/Engine/EditorBlueprintResources/StandardMacros.IsValid` (`self.HostGameMenuWB`)
    (:`Is Valid`
      _)
    (:`Is Not Valid`
      (bind _returnvalue (`|CreateWidget` "/Game/MP_SK/UI/MainMenu/HostGameMenu.HostGameMenu_C" (`GameplayStatics.GetPlayerController` 0)))
      (bind _output_get (set `self.HostGameMenuWB` _returnvalue))))
  (`UserWidget.AddToViewport` _output_get 0) ; And add the MainMenu to the Viewport
)

(event `ShowServerBrowserMenu`
  ;[0 0.5871 1] MENU
  ;;[1 1 1] Display ServerBrovser Menu Widget
  (`WidgetLayoutLibrary.RemoveAllWidgets`)
  (`/Engine/EditorBlueprintResources/StandardMacros.IsValid` (`self.ServerBrowserMenuWB`)
    (:`Is Valid`
      _)
    (:`Is Not Valid`
      (bind _returnvalue (`|CreateWidget` "/Game/MP_SK/UI/MainMenu/ServerBrowserMenu.ServerBrowserMenu_C" (`GameplayStatics.GetPlayerController` 0)))
      (bind _output_get (set `self.ServerBrowserMenuWB` _returnvalue))))
  (`UserWidget.AddToViewport` _output_get 0) ; And add the MainMenu to the Viewport
)

(event `ShowCharacterMenu`
  ;[0 0.5871 1] MENU
  ;;[1 1 1] Display Character Menu Widget
  (`WidgetLayoutLibrary.RemoveAllWidgets`)
  (`/Engine/EditorBlueprintResources/StandardMacros.IsValid` (`self.CharacterSettingsWB`)
    (:`Is Valid`
      _)
    (:`Is Not Valid`
      (bind _returnvalue (`|CreateWidget` "/Game/MP_SK/UI/MainMenu/CharacterSettings.CharacterSettings_C" (`GameplayStatics.GetPlayerController` 0)))
      (bind _output_get (set `self.CharacterSettingsWB` _returnvalue))))
  (`UserWidget.AddToViewport` _output_get 0) ; And add the MainMenu to the Viewport
)

(event `ShowSettingsMenu`
  ;[0 0.5871 1] MENU
  ;;[1 1 1] Display Character Menu Widget
  (`WidgetLayoutLibrary.RemoveAllWidgets`)
  (`/Engine/EditorBlueprintResources/StandardMacros.IsValid` (`self.SettingsWB`)
    (:`Is Valid`
      _)
    (:`Is Not Valid`
      (bind _returnvalue (`|CreateWidget` "/Game/MP_SK/UI/MainMenu/SettingsMenu.SettingsMenu_C" (`GameplayStatics.GetPlayerController` 0)))
      (bind _output_get (set `self.SettingsWB` _returnvalue))))
  (`UserWidget.AddToViewport` _output_get 0) ; And add the MainMenu to the Viewport
)