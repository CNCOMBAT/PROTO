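; Lobby game mode that manages players, chat and match start in a multiplayer lobby.
; BeginPlay, login and logout share one path that refreshes every LobbyPC's player list and posts "joined" chat messages, using Steam names when available.
; When two or more players are all ready, it cuts the LobbyGS countdown to one second.
; Match start saves player settings, shows loading screens and server-travels to the GameInstance map.
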(event `self.ReceiveBeginPlay`
  ;[1 1 1] New Player PostLogIn. Updage Player Lists on all clients
  (bind _outactors (`GameplayStatics.GetAllActorsOfClass` "/Game/MP_SK/Blueprints/Lobby/LobbyPC.LobbyPC_C" :!label _label))
  (for _array_element _outactors
    (bind _aslobby_pc (cast `/Game/MP_SK/Blueprints/Lobby/LobbyPC` _array_element :!pure true))
    (`/Game/MP_SK/Blueprints/Lobby/LobbyPC.CL_GeneratePlayerLists` _aslobby_pc)
    (bind _team (message `/Game/MP_SK/Blueprints/Interfaces/BasePS.IF_GetTeam` _aslobby_pc))
    (if (`AdvancedSessionsLibrary.HasOnlineSubsystem` "STEAM")
      (`KismetSystemLibrary.Delay` 1.0)
      (bind _returnvalue (`AdvancedSteamFriendsLibrary.GetSteamPersonaName` (`AdvancedSessionsLibrary.GetUniqueNetID` _aslobby_pc)))
      (`self.SRV_AddChatMessage` "Console" (`KismetStringLibrary.Concat_StrStr` "--> " _returnvalue " Joined the lobby.") (make `SlateColor` (struct :`G` 1.0 :`B` 0.992927 :`A` 1.0)) _team)
      (else
        (`KismetSystemLibrary.Delay` 1.0)
        (`self.SRV_AddChatMessage` "Console" (`KismetStringLibrary.Concat_StrStr` "--> " (`KismetSystemLibrary.GetDisplayName` _aslobby_pc) " Joined the lobby.") (make `SlateColor` (struct :`G` 1.0 :`B` 0.992927 :`A` 1.0)) _team)))))

(event `self.K2_PostLogin`
  (params (NewPlayer :type "PlayerController Object Reference"))
  ;[1 1 1] New Player PostLogIn. Updage Player Lists on all clients
  (goto _label))

(event `self.K2_OnLogout`
  (params (ExitingController :type "Controller Object Reference"))
  ;[1 1 1] Update Player Lists on all clients when some player Logout
  (goto _label))

(event `E_UpdatePlayerLists`
  ;[1 1 1] Update players lists on all clients
  (bind _outactors (`GameplayStatics.GetAllActorsOfClass` "/Game/MP_SK/Blueprints/Lobby/LobbyPC.LobbyPC_C"))
  (for _array_element _outactors
    (`/Game/MP_SK/Blueprints/Lobby/LobbyPC.CL_GeneratePlayerLists` (cast `/Game/MP_SK/Blueprints/Lobby/LobbyPC` _array_element :!pure true))))

(event `E_InitPlayersClass`
  ;[1 1 1] Init Class for everyone when updating server settings
  (`KismetSystemLibrary.Delay` 0.2)
  (for _array_element (`self.AllPlayerControllers`)
    (bind _aslobby_pc (cast `/Game/MP_SK/Blueprints/Lobby/LobbyPC` _array_element))
    (`/Game/MP_SK/Blueprints/Lobby/LobbyPC.CL_InitClass` _aslobby_pc)))

(event `E_IsAllReady`
  (bind _playerarray (`GameStateBase.PlayerArray` (`GameplayStatics.GetGameState`)))
  ;[1 1 1] Check is All players are ready and if YES - set Minutes = 0 and seconds = 5 in GameState
  (for _array_element _playerarray
    (bind _aslobby_ps (cast `/Game/MP_SK/Blueprints/Lobby/LobbyPS` _array_element))
    (if (`/Game/MP_SK/Blueprints/Lobby/LobbyPS.IsReady` _aslobby_ps)
      (set `self.AllReady` true)
      (else
        (set `self.AllReady` false)
        (break))))
  (if (and (`self.AllReady`) (>= (`KismetArrayLibrary.Array_Length` _playerarray) 2))
    (bind _aslobby_gs (cast `/Game/MP_SK/Blueprints/Lobby/LobbyGS` (`GameplayStatics.GetGameState`)))
    (set `/Game/MP_SK/Blueprints/Lobby/LobbyGS.minutes` 0 _aslobby_gs)
    (set `/Game/MP_SK/Blueprints/Lobby/LobbyGS.seconds` 1 _aslobby_gs)))

(event `E_StartMatch`
  ;[0 1 0.05329] Start Match
  (bind _outactors (`GameplayStatics.GetAllActorsOfClass` "/Game/MP_SK/Blueprints/Lobby/LobbyPC.LobbyPC_C"))
  (for _array_element _outactors
    (bind _aslobby_pc (cast `/Game/MP_SK/Blueprints/Lobby/LobbyPC` _array_element))
    (`/Game/MP_SK/Blueprints/Lobby/LobbyPC.CL_SavePlayerSettingsInGI` _aslobby_pc)
    (`/Game/MP_SK/Blueprints/Lobby/LobbyPC.CL_ShowLobbyLoadingScreen` _aslobby_pc))
  (`KismetSystemLibrary.ExecuteConsoleCommand` (`self.F_ServerTraverCommand`) (`GameplayStatics.GetPlayerController` 0)))

(event `SRV_AddChatMessage`
  (params (SenderName :type String) (Message :type String) (SenderColor :type "SlateColor Structure") (team4colorCHAT :type Integer))
  ;[1 1 1] Add chat message in ChatBox on all clients
  (bind _outactors (`GameplayStatics.GetAllActorsOfClass` "/Game/MP_SK/Blueprints/Lobby/LobbyPC.LobbyPC_C"))
  (for _array_element _outactors
    (bind _aslobby_pc (cast `/Game/MP_SK/Blueprints/Lobby/LobbyPC` _array_element))
    (`/Engine/EditorBlueprintResources/StandardMacros.IsValid` _aslobby_pc
      (:`Is Valid`
        (`/Game/MP_SK/Blueprints/Lobby/LobbyPC.CL_GetChatMessage` _aslobby_pc SenderName Message SenderColor team4colorCHAT)))))

(fn `F_ServerTraverCommand`
  (returns (`Travel command` :type String))
  (bind _asmain_gi (cast `/Game/MP_SK/Blueprints/MainGI` (`GameplayStatics.GetGameInstance`)))
  (return (`KismetStringLibrary.Concat_StrStr` "servertravel " (`/Game/MP_SK/Blueprints/MainGI.Mapname` _asmain_gi))))

(fn `UserConstructionScript`)