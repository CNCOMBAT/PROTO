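; Lobby GameState that holds the server and match settings for a multiplayer lobby and runs the countdown to match start.
; On BeginPlay the authority copies settings from MainGI and starts a looping one-second timer.
; When the countdown expires, the timer pauses and the server tells LobbyGM to start the match.
; SRV events store lobby edits and write settings back to MainGI, except UnevenTeams, which stays in the GameState.
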(event `self.ReceiveBeginPlay`
  ;[1 1 1] Save setting from main game instance in GameState
  (`/Engine/EditorBlueprintResources/ActorMacros.Switch Has Authority`
    (:`Authority`
      (bind _asmain_gi (cast `/Game/MP_SK/Blueprints/MainGI` (`GameplayStatics.GetGameInstance`)))
      (bind _output_get (set `self.MainGI` _asmain_gi))
      (`self.F_InitServerSettings` (`/Game/MP_SK/Blueprints/MainGI.IMaxPlayers` _output_get) (`/Game/MP_SK/Blueprints/MainGI.IRoundTime` _output_get) (`/Game/MP_SK/Blueprints/MainGI.IFriendlyFire` _output_get) (`/Game/MP_SK/Blueprints/MainGI.IServerName` _output_get) (`/Game/MP_SK/Blueprints/MainGI.IGameMode` _output_get) (`/Game/MP_SK/Blueprints/MainGI.AssaultClass` _output_get) (`/Game/MP_SK/Blueprints/MainGI.MedicClass` _output_get) (`/Game/MP_SK/Blueprints/MainGI.SniperClass` _output_get) (`/Game/MP_SK/Blueprints/MainGI.IMapIndex` _output_get))
      (bind _returnvalue (`KismetSystemLibrary.K2_SetTimer` null "StartTimerAndMaybeStartGame" 1.0 true))
      (set `self.LobbyTimerHandle` _returnvalue))))

(event `SRV_SaveSettingsInGI`
  ;[1 1 1] Save Server and Player settings to Game Instance
  (`self.SaveSettingsInGI` (`self.GSMaxPlayers`) (`self.GSRoundTime`) (`self.GSFriendlyFire`) (`self.GSServerName`) (`self.GSGameMode`) (`self.AssaultClass`) (`self.MedicClass`) (`self.SniperClass`) (`self.MapIndex`) (`self.GameModeId`)))

(event `SRV_SaveSettingsFromLobby`
  (params (MapIndex :type Integer) (GSGameMode :type String) (GameModeId :type Integer) (GSRoundTime :type String) (GSFriendlyFire :type Boolean) (AssaultClass :type Boolean) (MedicClass :type Boolean) (SniperClass :type Boolean) (Uneven_Teams :type Boolean))
  ;[1 1 1] Save settings from lobby
  (set `self.MapIndex` MapIndex)
  (set `self.GSGameMode` GSGameMode)
  (set `self.GameModeId` GameModeId)
  (set `self.GSRoundTime` GSRoundTime)
  (set `self.GSFriendlyFire` GSFriendlyFire)
  (set `self.AssaultClass` AssaultClass)
  (set `self.MedicClass` MedicClass)
  (set `self.SniperClass` SniperClass)
  (set `self.Uneven_Teams` Uneven_Teams))

(fn `F_InitServerSettings`
  (params (MaxPlayers :type String) (RoundTime :type String) (FriendlyFire :type Boolean) (ServerName :type String) (`Game-Mode` :type String) (AssaultClass :type Boolean) (MedicClass :type Boolean) (SniperClass :type Boolean) (MapIndex :type Integer))
  (set `self.GSMaxPlayers` MaxPlayers)
  (set `self.GSRoundTime` RoundTime)
  (set `self.GSFriendlyFire` FriendlyFire)
  (set `self.GSServerName` ServerName)
  (set `self.GSGameMode` `Game-Mode`)
  (set `self.GSMapName` "")
  (set `self.AssaultClass` AssaultClass)
  (set `self.MedicClass` MedicClass)
  (set `self.SniperClass` SniperClass)
  (set `self.MapIndex` MapIndex))

(fn `SaveSettingsInGI`
  (params (MaxPlayers :type String) (RoundTime :type String) (FriendlyFire :type Boolean) (ServerName :type String) (`Game-Mode` :type String) (AssaultClass :type Boolean) (MedicClass :type Boolean) (SniperClass :type Boolean) (MapIndex :type Integer) (GameModeId :type Integer))
  (bind _maingi (`self.MainGI`))
  (set `/Game/MP_SK/Blueprints/MainGI.IMaxPlayers` MaxPlayers _maingi)
  (set `/Game/MP_SK/Blueprints/MainGI.IRoundTime` RoundTime _maingi)
  (set `/Game/MP_SK/Blueprints/MainGI.IFriendlyFire` FriendlyFire _maingi)
  (set `/Game/MP_SK/Blueprints/MainGI.IServerName` ServerName _maingi)
  (set `/Game/MP_SK/Blueprints/MainGI.IGameMode` `Game-Mode` _maingi)
  (set `/Game/MP_SK/Blueprints/MainGI.AssaultClass` AssaultClass _maingi)
  (set `/Game/MP_SK/Blueprints/MainGI.MedicClass` MedicClass _maingi)
  (set `/Game/MP_SK/Blueprints/MainGI.SniperClass` SniperClass _maingi)
  (set `/Game/MP_SK/Blueprints/MainGI.IMapIndex` MapIndex _maingi)
  (set `/Game/MP_SK/Blueprints/MainGI.GameModeId` GameModeId _maingi))

(fn `StartTimerAndMaybeStartGame`
  (bind _minutes (`self.minutes`))
  (if (and (== (`self.seconds`) 60) (== (`self.minutes`) 0))
    ;[1 0.03503 0] Pause Timer and Start Match on time expired
    (`KismetSystemLibrary.K2_PauseTimerHandle` (`self.LobbyTimerHandle`))
    (if (`KismetSystemLibrary.IsServer`)
      (`/Game/MP_SK/Blueprints/Lobby/LobbyGM.E_StartMatch` (cast `/Game/MP_SK/Blueprints/Lobby/LobbyGM` (`GameplayStatics.GetGameMode`) :!pure true)))
    (else
      (bind _output_get (set `self.seconds` (- (`self.seconds`) 1)))
      (if (== _output_get 0)
        (set `self.seconds` 60)
        (if (!= _minutes 0)
          (set `self.minutes` (- _minutes 1)))))))

(fn `UserConstructionScript`)