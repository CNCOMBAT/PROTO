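; Lobby player controller that runs each player's team, class, ready state and chat in the multiplayer lobby.
; On local start it creates the lobby widget, auto-balances the team and, after delays, replaces disallowed classes and refreshes class buttons.
; SRV events write to LobbyPS or forward to LobbyGM.
; CL events rebuild team lists, show chat and loading screen, and save team and class to the GameInstance.
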(event `remove widgets`
  ;[1 0.06418 0] Begin Play. Create Lobby widget
  (`WidgetLayoutLibrary.RemoveAllWidgets`))

(event `CL_SavePlayerSettingsInGI`
  (bind _maingi (`self.MainGI`))
  ;[1 1 1] Save PlayerTeam and PlayerClass from PlayerState in GameInstance
  (bind _aslobby_ps (cast `/Game/MP_SK/Blueprints/Lobby/LobbyPS` (`self.PlayerState`)))
  (set `/Game/MP_SK/Blueprints/MainGI.PawnClass` (`/Game/MP_SK/Blueprints/Lobby/LobbyPS.PawnClass` _aslobby_ps) _maingi)
  (set `/Game/MP_SK/Blueprints/MainGI.PlayerTeam` (`/Game/MP_SK/Blueprints/Lobby/LobbyPS.Team` _aslobby_ps) _maingi))

(event `SRV_UpdatePlayerClassForAll`
  ;[1 1 1] Update player class for all
  (bind _aslobby_gm (cast `/Game/MP_SK/Blueprints/Lobby/LobbyGM` (`GameplayStatics.GetGameMode`)))
  (`/Game/MP_SK/Blueprints/Lobby/LobbyGM.E_InitPlayersClass` _aslobby_gm))

(event `self.ReceiveBeginPlay`
  ;[1 0.06418 0] Begin Play. Create Lobby widget
  (`|ExecutionSequence`
    (:`then_0`
      (`self.remove widgets`))
    (:`then_1`
      (bind _asmain_gi (cast `/Game/MP_SK/Blueprints/MainGI` (`GameplayStatics.GetGameInstance`)))
      (bind _output_get (set `self.MainGI` _asmain_gi))
      (set `/Game/MP_SK/Blueprints/MainGI.AmIFromLobby` true _output_get))
    (:`then_2`
      (if (`self.IsLocalPlayerController`)
        (`self.SRV_SetTeam`)))
    (:`then_3`
      (if (`self.IsLocalPlayerController`)
        (`self.E_CreateLobbyWB`)
        (`KismetSystemLibrary.Delay` 2.0)
        (`self.F_SetupReferences`)
        (`self.CL_InitClass`)))))

(event `CL_InitClass`
  (bind _lobbywb (`self.LobbyWB`))
  (bind _medicclassbutton (`/Game/MP_SK/UI/Lobby/Lobby.MedicClassButton` _lobbywb))
  (bind _sniperclassbutton (`/Game/MP_SK/UI/Lobby/Lobby.SniperClassButton` _lobbywb))
  (bind _assaultclassbutton (`/Game/MP_SK/UI/Lobby/Lobby.AssaultClassButton` _lobbywb))
  ;[0.2322 1 0] Init Player Class!
  (`|ExecutionSequence`
    (:`then_0`
      (`KismetSystemLibrary.Delay` 1.0)
      (bind _aslobby_gs (cast `/Game/MP_SK/Blueprints/Lobby/LobbyGS` (`GameplayStatics.GetGameState`)))
      (if (`/Game/MP_SK/Blueprints/Lobby/LobbyGS.AssaultClass` _aslobby_gs)
        ;;[1 1 1] Set assault class only if 1. assault class is allowed. AND 2. You are sniper and sniper class not allowed OR you are medic and medic class is not allowed
        (if (and (not (`/Game/MP_SK/Blueprints/Lobby/LobbyGS.MedicClass` (`self.LobbyGS`))) (== (`/Game/MP_SK/Blueprints/Lobby/LobbyPS.PawnClass` (`self.LobbyPS`)) 1))
          (`self.SRV_SetAssaultClass` :!label _label)
          (elif (and (not (`/Game/MP_SK/Blueprints/Lobby/LobbyGS.SniperClass` (`self.LobbyGS`))) (== (`/Game/MP_SK/Blueprints/Lobby/LobbyPS.PawnClass` (`self.LobbyPS`)) 2))
            (goto _label)))
        (elif (`/Game/MP_SK/Blueprints/Lobby/LobbyGS.MedicClass` _aslobby_gs)
          ;;[1 1 1] Set medic class only if 1. medic class is allowed. AND 2. You are medic and medic class not allowed OR you are assault and assault class is not allowed
          (if (and (not (`/Game/MP_SK/Blueprints/Lobby/LobbyGS.AssaultClass` (`self.LobbyGS`))) (== (`/Game/MP_SK/Blueprints/Lobby/LobbyPS.PawnClass` (`self.LobbyPS`)) 0))
            (`self.SRV_SetMedicClass` :!label _label_2)
            (elif (and (not (`/Game/MP_SK/Blueprints/Lobby/LobbyGS.SniperClass` (`self.LobbyGS`))) (== (`/Game/MP_SK/Blueprints/Lobby/LobbyPS.PawnClass` (`self.LobbyPS`)) 2))
              (goto _label_2)))
          (elif (`/Game/MP_SK/Blueprints/Lobby/LobbyGS.SniperClass` _aslobby_gs)
            ;;[1 1 1] Set siper class only if 1. sniper class is allowed. AND 2. You are medic and medic class not allowed OR you are assault and assault class is not allowed
            (if (and (not (`/Game/MP_SK/Blueprints/Lobby/LobbyGS.MedicClass` (`self.LobbyGS`))) (== (`/Game/MP_SK/Blueprints/Lobby/LobbyPS.PawnClass` (`self.LobbyPS`)) 1))
              (`self.SRV_SetSniperClass` :!label _label_3)
              (elif (and (not (`/Game/MP_SK/Blueprints/Lobby/LobbyGS.AssaultClass` (`self.LobbyGS`))) (== (`/Game/MP_SK/Blueprints/Lobby/LobbyPS.PawnClass` (`self.LobbyPS`)) 0))
                (goto _label_3)))))))
    (:`then_1`
      ;;[1 1 1] Do not allow players cnange class when we are updating Server and allowed classes settings
      (`Widget.SetIsEnabled` (`/Game/MP_SK/UI/Lobby/Lobby.AssaultClassButton` (`self.LobbyWB`)) false)
      (`Widget.SetIsEnabled` (`/Game/MP_SK/UI/Lobby/Lobby.MedicClassButton` (`self.LobbyWB`)) false)
      (`Widget.SetIsEnabled` (`/Game/MP_SK/UI/Lobby/Lobby.SniperClassButton` (`self.LobbyWB`)) false)
      ;;[1 1 1] Update buttons state (enabled/disabled) in LobbyWB
      (`KismetSystemLibrary.Delay` 1.5)
      (if (and (`/Game/MP_SK/Blueprints/Lobby/LobbyGS.AssaultClass` (`self.LobbyGS`)) (!= (`/Game/MP_SK/Blueprints/Lobby/LobbyPS.PawnClass` (`self.LobbyPS`)) 0))
        (`Widget.SetIsEnabled` _assaultclassbutton true)
        (else
          (`Widget.SetIsEnabled` _assaultclassbutton false)))
      (if (and (`/Game/MP_SK/Blueprints/Lobby/LobbyGS.MedicClass` (`self.LobbyGS`)) (!= (`/Game/MP_SK/Blueprints/Lobby/LobbyPS.PawnClass` (`self.LobbyPS`)) 1))
        (`Widget.SetIsEnabled` _medicclassbutton true)
        (else
          (`Widget.SetIsEnabled` _medicclassbutton false)))
      (if (and (`/Game/MP_SK/Blueprints/Lobby/LobbyGS.SniperClass` (`self.LobbyGS`)) (!= (`/Game/MP_SK/Blueprints/Lobby/LobbyPS.PawnClass` (`self.LobbyPS`)) 2))
        (`Widget.SetIsEnabled` _sniperclassbutton true)
        (else
          (`Widget.SetIsEnabled` _sniperclassbutton false))))))

(event `SRV_SendChatMessage`
  (params (SenderName :type String) (Message :type String) (SenderColor :type "SlateColor Structure") (team4colorCHAT :type Integer))
  ;[0 1 0.31] Send and Get chat message in Lobby
  (bind _aslobby_gm (cast `/Game/MP_SK/Blueprints/Lobby/LobbyGM` (`GameplayStatics.GetGameMode`)))
  (`/Game/MP_SK/Blueprints/Lobby/LobbyGM.SRV_AddChatMessage` _aslobby_gm SenderName Message SenderColor team4colorCHAT))

(event `join team red`
  (bind _aslobby_gm (cast `/Game/MP_SK/Blueprints/Lobby/LobbyGM` (`GameplayStatics.GetGameMode`) :!pure true))
  ;[1 1 1] Set Player team
  (bind _aslobby_ps (cast `/Game/MP_SK/Blueprints/Lobby/LobbyPS` (`self.PlayerState`) :!label _label_4))
  (set `/Game/MP_SK/Blueprints/Lobby/LobbyPS.Team` 0 _aslobby_ps)
  (set `/Game/MP_SK/Blueprints/Lobby/LobbyGM.RedTeamPlayersCount` (+ (`/Game/MP_SK/Blueprints/Lobby/LobbyGM.RedTeamPlayersCount` _aslobby_gm) 1) _aslobby_gm))

(event `SRV_SetTeam`
  (bind _aslobby_gm (cast `/Game/MP_SK/Blueprints/Lobby/LobbyGM` (`GameplayStatics.GetGameMode`) :!pure true))
  ;[1 1 1] Set Player team
  (if (>= (`/Game/MP_SK/Blueprints/Lobby/LobbyGM.BlueTeamPlayersCount` _aslobby_gm) (`/Game/MP_SK/Blueprints/Lobby/LobbyGM.RedTeamPlayersCount` _aslobby_gm))
    (goto _label_4)
    (else
      (bind _aslobby_ps (cast `/Game/MP_SK/Blueprints/Lobby/LobbyPS` (`self.PlayerState`) :!label _label_5))
      (set `/Game/MP_SK/Blueprints/Lobby/LobbyPS.Team` 1 _aslobby_ps)
      (set `/Game/MP_SK/Blueprints/Lobby/LobbyGM.BlueTeamPlayersCount` (+ (`/Game/MP_SK/Blueprints/Lobby/LobbyGM.BlueTeamPlayersCount` _aslobby_gm) 1) _aslobby_gm))))

(event `CL_GetChatMessage`
  (params (SenderName :type String) (Message :type String) (SenderColor :type "SlateColor Structure") (team4colorCHAT :type Integer))
  (bind _lobbywb (`self.LobbyWB`))
  (bind _chatscrollbox (`/Game/MP_SK/UI/Lobby/Lobby.ChatScrollBox` _lobbywb))
  ;[0 1 0.31] Send and Get chat message in Lobby
  (bind _returnvalue (`|CreateWidget` "/Game/MP_SK/UI/Lobby/AdditionalLobbyWidgets/LobbyChatMessage.LobbyChatMessage_C" (`GameplayStatics.GetPlayerController` 0) SenderName Message SenderColor team4colorCHAT))
  (`PanelWidget.AddChild` _chatscrollbox _returnvalue)
  (`ScrollBox.ScrollToEnd` _chatscrollbox)
  (`EditableTextBox.SetText` (`/Game/MP_SK/UI/Lobby/Lobby.chatMessage` _lobbywb) ""))

(event `join team blue`
  ;[1 1 1] Set Player team
  (goto _label_5))

(event `SRV_SetAssaultClass`
  ;[0 0.1401 1] Change Class
  ;;[1 1 1] Set Assault Class
  (bind _aslobby_ps (cast `/Game/MP_SK/Blueprints/Lobby/LobbyPS` (`self.PlayerState`)))
  (set `/Game/MP_SK/Blueprints/Lobby/LobbyPS.PawnClass` 0 _aslobby_ps)
  (set `/Game/MP_SK/Blueprints/Lobby/LobbyPS.ClassImg` (make `SlateBrush` (37.0 40.0) (struct) (struct :`SpecifiedColor` (struct :`R` 1.0 :`G` 1.0 :`B` 1.0 :`A` 1.0) :`ColorUseRule` "UseColor_Specified") "/Game/MP_SK/UI/UI_textures/assault_class_icon1.assault_class_icon1") _aslobby_ps))

(event `SRV_UpdatePlayerLists`
  ;[1 1 1] Update player lists for all players, on player class and team change and wneh new player joins the game
  (`/Game/MP_SK/Blueprints/Lobby/LobbyGM.E_UpdatePlayerLists` (cast `/Game/MP_SK/Blueprints/Lobby/LobbyGM` (`GameplayStatics.GetGameMode`) :!pure true)))

(event `SRV_SetMedicClass`
  ;[0 0.1401 1] Change Class
  ;;[1 1 1] Set Medic Class
  (bind _aslobby_ps (cast `/Game/MP_SK/Blueprints/Lobby/LobbyPS` (`self.PlayerState`)))
  (set `/Game/MP_SK/Blueprints/Lobby/LobbyPS.PawnClass` 1 _aslobby_ps)
  (set `/Game/MP_SK/Blueprints/Lobby/LobbyPS.ClassImg` (make `SlateBrush` (37.0 40.0) (struct) (struct :`SpecifiedColor` (struct :`R` 1.0 :`G` 1.0 :`B` 1.0 :`A` 1.0) :`ColorUseRule` "UseColor_Specified") "/Game/MP_SK/UI/UI_textures/medic_class_icon.medic_class_icon") _aslobby_ps))

(event `E_CreateLobbyWB`
  ;[1 1 1] Create lobby widget
  (bind _returnvalue (`|CreateWidget` "/Game/MP_SK/UI/Lobby/Lobby.Lobby_C" self))
  (bind _output_get (set `self.LobbyWB` _returnvalue))
  (`UserWidget.AddToViewport` _output_get 0)
  (set `self.bShowMouseCursor` true))

(event `SRV_SetSniperClass`
  ;[0 0.1401 1] Change Class
  ;;[1 1 1] Set Sniper Class
  (bind _aslobby_ps (cast `/Game/MP_SK/Blueprints/Lobby/LobbyPS` (`self.PlayerState`)))
  (set `/Game/MP_SK/Blueprints/Lobby/LobbyPS.PawnClass` 2 _aslobby_ps)
  (set `/Game/MP_SK/Blueprints/Lobby/LobbyPS.ClassImg` (make `SlateBrush` (37.0 40.0) (struct) (struct :`SpecifiedColor` (struct :`R` 1.0 :`G` 1.0 :`B` 1.0 :`A` 1.0) :`ColorUseRule` "UseColor_Specified") "/Game/MP_SK/UI/UI_textures/sniper_class_icon1.sniper_class_icon1") _aslobby_ps))

(event `SRV_CheckIsAllReady`
  ;[1 1 1] Check is all ready
  (bind _aslobby_gm (cast `/Game/MP_SK/Blueprints/Lobby/LobbyGM` (`GameplayStatics.GetGameMode`)))
  (`/Game/MP_SK/Blueprints/Lobby/LobbyGM.E_IsAllReady` _aslobby_gm))

(event `playsoundready`
  ;[0 0.1634 1] Toggle Ready
  (`GameplayStatics.SpawnSoundAtLocation` "/Game/audio/readyup.readyup" (0.0 0.0 0.0) (struct) 1.0 1.0 0.0 null null :!label _label_6)
  (`self.SRV_CheckIsAllReady` :!label _label_7))

(event `SRV_ToggleReady`
  ;[0 0.1634 1] Toggle Ready
  (bind _aslobby_ps (cast `/Game/MP_SK/Blueprints/Lobby/LobbyPS` (`self.PlayerState`)))
  (if (`/Game/MP_SK/Blueprints/Lobby/LobbyPS.IsReady` _aslobby_ps)
    (set `/Game/MP_SK/Blueprints/Lobby/LobbyPS.IsReady` false _aslobby_ps)
    (goto _label_7)
    (else
      (set `/Game/MP_SK/Blueprints/Lobby/LobbyPS.IsReady` true _aslobby_ps)
      (goto _label_6))))

(event `CL_ShowLobbyLoadingScreen`
  ;[1 1 1] Show loading screen
  (bind _returnvalue (`|CreateWidget` "/Game/MP_SK/UI/Lobby/AdditionalLobbyWidgets/LobbyLoadingScreen.LobbyLoadingScreen_C" self))
  (`UserWidget.AddToViewport` _returnvalue 0))

(event `CL_GeneratePlayerLists`
  (bind _lobbywb (`self.LobbyWB`))
  ;[0 1 0.953] Generate Player Lists. Red and blue teams
  (`KismetSystemLibrary.Delay` 1.0)
  (`/Engine/EditorBlueprintResources/StandardMacros.IsValid` (`self.LobbyWB`)
    (:`Is Valid`
      (`PanelWidget.ClearChildren` (`/Game/MP_SK/UI/Lobby/Lobby.RedTeamPlayersList` (`self.LobbyWB`)))
      (`PanelWidget.ClearChildren` (`/Game/MP_SK/UI/Lobby/Lobby.BlueTeamPlayersList` (`self.LobbyWB`)))
      (for _array_element (`GameStateBase.PlayerArray` (`GameplayStatics.GetGameState`))
        (bind _aslobby_ps (cast `/Game/MP_SK/Blueprints/Lobby/LobbyPS` _array_element :!pure true))
        (bind _returnvalue (`|CreateWidget` "/Game/MP_SK/UI/Lobby/AdditionalLobbyWidgets/PlayerInfoLine.PlayerInfoLine_C" self (`PlayerState.PlayerId` _aslobby_ps)))
        (switch `int` (`/Game/MP_SK/Blueprints/Lobby/LobbyPS.Team` _aslobby_ps)
          (:`0`
            (`PanelWidget.AddChild` (`/Game/MP_SK/UI/Lobby/Lobby.RedTeamPlayersList` _lobbywb) _returnvalue))
          (:`1`
            (`PanelWidget.AddChild` (`/Game/MP_SK/UI/Lobby/Lobby.BlueTeamPlayersList` _lobbywb) _returnvalue)))))))

(fn `F_SetupReferences`
  (set `self.LobbyGS` (cast `/Game/MP_SK/Blueprints/Lobby/LobbyGS` (`GameplayStatics.GetGameState`) :!pure true))
  (set `self.LobbyPS` (cast `/Game/MP_SK/Blueprints/Lobby/LobbyPS` (`self.PlayerState`) :!pure true)))

(fn `UserConstructionScript`)